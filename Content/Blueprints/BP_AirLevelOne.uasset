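; BP_AirLevelOne is a trigger zone that drives heat updates on the player's BP_PC pawn.
; Any overlap with BoxForAir calls Heat, which sets HeatBegin after a 30-second delay.
; While the flag is set, Tick calls UpdateHeat on player pawn 0 every frame.
; Ending the overlap clears the flag but does not cancel a pending delay, so heating can still begin afterward.
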(event OnComponentBeginOverlap(BoxForAir)
  (params (OverlappedComponent :type Primitive%20Component%20Object%20Reference) (OtherActor :type Actor%20Object%20Reference) (OtherComp :type Primitive%20Component%20Object%20Reference) (OtherBodyIndex :type Integer) (bFromSweep :type Boolean) (SweepResult :type Hit%20Result%20Structure%20%28by%20ref%29))
  (CallFunction|Heat))

(event OnComponentEndOverlap(BoxForAir)
  (params (OverlappedComponent :type Primitive%20Component%20Object%20Reference) (OtherActor :type Actor%20Object%20Reference) (OtherComp :type Primitive%20Component%20Object%20Reference) (OtherBodyIndex :type Integer))
  (Variables|Default|SetHeatBegin false))

(event Custom|Heat
  (Utilities|FlowControl|Delay 3e+01)
  (Variables|Default|SetHeatBegin true))

(event EventBeginPlay)

(event Collision|EventActorBeginOverlap
  (params (OtherActor :type Actor%20Object%20Reference)))

(event EventTick
  (params (DeltaSeconds :type Float%20%28single-precision%29))
  (if (Variables|Default|GetHeatBegin)
    (bind _asbp_pc (Utilities|Casting|CastToBP_PC (Game|Player|GetPlayerPawn 0)))
    (Default|UpdateHeat _asbp_pc)))

(fn ConstructionScript)
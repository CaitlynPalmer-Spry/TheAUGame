(event EventBeginPlay
  ;[0.15 0.15 0.15 0.5] Create Inventory
  (bind _returnvalue (UserInterface|CreateWidget "/Game/UI/UI_Inventory.UI_Inventory_C"))
  (Variables|Default|SetInventoryWidget _returnvalue)
  (Utilities|Array|Resize (Variables|Default|GetItems) 10)
  (Default|LoadInventory (Variables|Default|GetInventoryWidget) self))

(event EventTick
  (params (DeltaSeconds :type Float%20%28single-precision%29)))

(event Input|KeyboardEvents|I
  (params (Key :type Key%20Structure :default "None"))
  (bind _returnvalue (Game|GetPlayerController 0))
  (bind _returnvalue_2 (Game|GetPlayerController 0))
  (bind _inventorywidget (Variables|Default|GetInventoryWidget))
  ;[0.15 0.15 0.15 0.5] Open Inventory
  (:Pressed
    (if (Widget|IsVisible (Variables|Default|GetInventoryWidget))
      (Widget|RemovefromParent _inventorywidget)
      (Variables|/Script/Engine.PlayerController|SetbShowMouseCursor _returnvalue_2 false)
      (Input|SetInputModeGameOnly _returnvalue_2 false)
      (else
        (Variables|/Script/Engine.PlayerController|SetbShowMouseCursor _returnvalue true)
        (Input|SetInputModeGameandUI _returnvalue 0 "DoNotLock" true false)
        (UserInterface|Viewport|AddtoViewport _inventorywidget 0)))))

(event Input|KeyboardEvents|E
  (params (Key :type Key%20Structure :default "None"))
  (bind _returnvalue (Game|Player|GetPlayerPawn 0))
  (bind _returnvalue_2 (Transformation|GetActorLocation _returnvalue))
  ;[0.15 0.15 0.15 0.5] Pick up items
  (:Pressed
    (bind _outhit (Collision|SphereTraceByChannel _returnvalue_2 _returnvalue_2 6e+01 "TraceTypeQuery3" false 0 "None"))
    (bind _asbp_item (Utilities|Casting|CastToBP_Item (.HitActor (Collision|BreakHitResult _outhit))))
    (for (_array_element _array_index) (Variables|Default|GetItems)
      (Utilities|IsValid _asbp_item
        (:Is%20Valid
          (if (Math|Boolean|ANDBoolean (Utilities|Enum|Equal(Enum) (.Name (Utilities|Struct|BreakS_ItemStructure _array_element)) (.Name (Utilities|Struct|BreakS_ItemStructure (Variables|/Game/Assets/2DItems/BP_Item.BP_Item_C|GetItem _asbp_item)))) (.Stackable (Utilities|Struct|BreakS_ItemStructure (Variables|/Game/Assets/2DItems/BP_Item.BP_Item_C|GetItem _asbp_item))) (<= (+ (.Quantity (Utilities|Struct|BreakS_ItemStructure _array_element)) (.Quantity (Utilities|Struct|BreakS_ItemStructure (Variables|/Game/Assets/2DItems/BP_Item.BP_Item_C|GetItem _asbp_item)))) 64))
            (Utilities|Array|SetArrayElem (Variables|Default|GetItems) _array_index (Utilities|Struct|MakeS_ItemStructure (.name (Variables|/Game/Assets/2DItems/BP_Item.BP_Item_C|GetItem _asbp_item)) (.stackable (Variables|/Game/Assets/2DItems/BP_Item.BP_Item_C|GetItem _asbp_item)) (+ (.Quantity (Utilities|Struct|BreakS_ItemStructure _array_element)) (.Quantity (Utilities|Struct|BreakS_ItemStructure (Variables|/Game/Assets/2DItems/BP_Item.BP_Item_C|GetItem _asbp_item)))) (.thumbnail (Variables|/Game/Assets/2DItems/BP_Item.BP_Item_C|GetItem _asbp_item)) (.2d_item (Variables|/Game/Assets/2DItems/BP_Item.BP_Item_C|GetItem _asbp_item)) (.gramweight (Variables|/Game/Assets/2DItems/BP_Item.BP_Item_C|GetItem _asbp_item))))
            (Default|LoadInventory (Variables|Default|GetInventoryWidget) self :!label _label)
            (Actor|DestroyActor _asbp_item)
            (elif (== (.Quantity (Utilities|Struct|BreakS_ItemStructure _array_element)) 0)
              (Utilities|Array|SetArrayElem (Variables|Default|GetItems) _array_index (Variables|/Game/Assets/2DItems/BP_Item.BP_Item_C|GetItem _asbp_item))
              (goto _label))))))))
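; Actor that shows staged panning visuals, advancing through six Panning components as the player's hit count rises.
; Every Tick it casts the game instance to GI_PlayerData and switches on TimesHit.
; Each count from one to five hides the current stage component and shows the next, only undoing the immediately previous one.
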(event EventBeginPlay)

(event Collision|EventActorBeginOverlap
  (params (OtherActor :type Actor%20Object%20Reference)))

(event EventTick
  (params (DeltaSeconds :type Float%20%28single-precision%29))
  (bind _panning2 (Variables|Default|GetPanning2))
  (bind _panning4 (Variables|Default|GetPanning4))
  (bind _panning5 (Variables|Default|GetPanning5))
  (bind _panning3 (Variables|Default|GetPanning3))
  (bind _asgi_player_data (Utilities|Casting|CastToGI_PlayerData (Game|GetGameInstance)))
  (switch int (Variables|/Game/Blueprints/GI_PlayerData.GI_PlayerData_C|GetTimesHit _asgi_player_data)
    (:1
      (Rendering|SetVisibility (Variables|Default|GetPanning1) false false)
      (Rendering|SetVisibility _panning2 true false))
    (:2
      (Rendering|SetVisibility _panning2 false false)
      (Rendering|SetVisibility _panning3 true false))
    (:3
      (Rendering|SetVisibility _panning3 false false)
      (Rendering|SetVisibility _panning4 true false))
    (:4
      (Rendering|SetVisibility _panning4 false false)
      (Rendering|SetVisibility _panning5 true false))
    (:5
      (Rendering|SetVisibility _panning5 false false)
      (Rendering|SetVisibility (Variables|Default|GetPanning6) true false))))

(fn ConstructionScript)
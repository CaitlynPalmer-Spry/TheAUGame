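; BP_Note1 is a note actor for what appears to be a rhythm lane, travelling along Lane1 of the level's BP_Spline.
; It finds that spline actor on BeginPlay, and MoveNotes plays a Timeline rate-scaled by TimeToComplete.
; Each update maps the timeline alpha to spline distance and sets the actor's transform from local-space location and rotation, using the Sphere's relative scale.
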(event Custom|MoveNotes
  (bind _rythemspline (Variables|Default|GetRythemSpline))
  (bind _lane_1 (Variables|/Game/Blueprints/PanningBlueprints/BP_Spline.BP_Spline_C|GetLane_1 _rythemspline))
  (Components|Timeline|SetPlayRate (Variables|Default|GetTimeline) (/ 1.5 (Variables|Default|GetTimeToComplete)))
  (bind _newtrack_0 (Timeline|Timeline PlayFromStart)
    (:Update
      (Transformation|SetActorTransform (Math|Transform|MakeTransform (Spline|GetLocationatDistanceAlongSpline _lane_1 (Math|Float|Lerp 0.0 (Spline|GetSplineLength (Variables|/Game/Blueprints/PanningBlueprints/BP_Spline.BP_Spline_C|GetLane_1 (Variables|Default|GetRythemSpline))) _newtrack_0) "Local") (Spline|GetRotationatDistanceAlongSpline _lane_1 (Math|Float|Lerp 0.0 (Spline|GetSplineLength (Variables|/Game/Blueprints/PanningBlueprints/BP_Spline.BP_Spline_C|GetLane_1 (Variables|Default|GetRythemSpline))) _newtrack_0) "Local") (Variables|/Script/Engine.SceneComponent|GetRelativeScale3D (Variables|Default|GetSphere)))))))

(event EventBeginPlay
  (bind _returnvalue (Actor|GetActorOfClass "/Game/Blueprints/PanningBlueprints/BP_Spline.BP_Spline_C"))
  (Variables|Default|SetRythemSpline _returnvalue))

(fn ConstructionScript)
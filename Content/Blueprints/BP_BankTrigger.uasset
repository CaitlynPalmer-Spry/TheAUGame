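; BP_BankTrigger is a trigger actor that shows the bank button UI while something overlaps its box.
; On overlap begin it creates a UI_BankButton widget and adds it to the viewport, but only if GI_PlayerData's TutorialJoeEventNumber is past a set tutorial step.
; On overlap end it removes the stored widget.
; Neither overlap event filters which actor triggered it.
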(event OnComponentBeginOverlap(Box)
  (params (OverlappedComponent :type Primitive%20Component%20Object%20Reference) (OtherActor :type Actor%20Object%20Reference) (OtherComp :type Primitive%20Component%20Object%20Reference) (OtherBodyIndex :type Integer) (bFromSweep :type Boolean) (SweepResult :type Hit%20Result%20Structure%20%28by%20ref%29))
  (bind _asgi_player_data (Utilities|Casting|CastToGI_PlayerData (Game|GetGameInstance)))
  (if (> (Variables|/Game/Blueprints/GI_PlayerData.GI_PlayerData_C|GetTutorialJoeEventNumber _asgi_player_data) 18)
    (bind _returnvalue (UserInterface|CreateWidget "/Game/UI/UI_BankButton.UI_BankButton_C"))
    (bind _output_get (Variables|Default|SetBank _returnvalue))
    (UserInterface|Viewport|AddtoViewport _output_get 0)))

(event OnComponentEndOverlap(Box)
  (params (OverlappedComponent :type Primitive%20Component%20Object%20Reference) (OtherActor :type Actor%20Object%20Reference) (OtherComp :type Primitive%20Component%20Object%20Reference) (OtherBodyIndex :type Integer))
  (bind _bank (Variables|Default|GetBank))
  (Utilities|IsValid _bank
    (:Is%20Valid
      (Widget|RemovefromParent _bank))))

(event EventBeginPlay)

(event Collision|EventActorBeginOverlap
  (params (OtherActor :type Actor%20Object%20Reference)))

(event EventTick
  (params (DeltaSeconds :type Float%20%28single-precision%29)))

(fn ConstructionScript)
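; Camp trigger actor that randomly starts a bandit attack when something overlaps its Trigger component.
; Each overlap, with no check on the overlapping actor, has a one-in-four chance to show the UI_BanditQuiz widget and mouse cursor, reveal three idle bandits and set BanditAttackHappening in GI_PlayerData.
; Debug strings print either outcome, and a note marks pausing the character during the quiz as unresolved.
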(event OnComponentBeginOverlap(Trigger)
  (params (OverlappedComponent :type Primitive%20Component%20Object%20Reference) (OtherActor :type Actor%20Object%20Reference) (OtherComp :type Primitive%20Component%20Object%20Reference) (OtherBodyIndex :type Integer) (bFromSweep :type Boolean) (SweepResult :type Hit%20Result%20Structure%20%28by%20ref%29))
  (if (== (Math|Random|RandomInteger 4) 1)
    (bind _returnvalue (UserInterface|CreateWidget "/Game/UI/UI_BanditQuiz.UI_BanditQuiz_C"))
    (UserInterface|Viewport|AddtoViewport _returnvalue 0)
    (Development|PrintString "Triggered!")
    (Variables|/Script/Engine.PlayerController|SetbShowMouseCursor (Game|GetPlayerController 0) true)
    (Rendering|SetVisibility (Variables|Default|GetF_Idle_bandit2) true false)
    (Rendering|SetVisibility (Variables|Default|GetF_Idle_Bandit3) true false)
    (Rendering|SetVisibility (Variables|Default|GetF_Idle_bandit1) true false)
    (bind _asgi_player_data (Utilities|Casting|CastToGI_PlayerData (Game|GetGameInstance)))
    (Variables|/Game/Blueprints/GI_PlayerData.GI_PlayerData_C|SetBanditAttackHappening? _asgi_player_data true)
    (else
      (Development|PrintString "Not Triggered"))))

(event EventBeginPlay)

(event Collision|EventActorBeginOverlap
  (params (OtherActor :type Actor%20Object%20Reference)))

(event EventTick
  (params (DeltaSeconds :type Float%20%28single-precision%29)))

(fn ConstructionScript)
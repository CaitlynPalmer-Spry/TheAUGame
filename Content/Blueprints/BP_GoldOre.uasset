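; Gold ore actor that is mined away after being hit, then destroys itself.
; A hit on the Ore component sets a mining flag, which nothing in this Blueprint clears.
; While flagged, Tick calls Mine, whose Delay throttles the Health countdown to timed steps.
; At zero Health it prints a "Drop Items" placeholder and destroys the actor, with no item spawning yet.
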(event OnComponentHit(Ore)
  (params (HitComponent :type Primitive%20Component%20Object%20Reference) (OtherActor :type Actor%20Object%20Reference) (OtherComp :type Primitive%20Component%20Object%20Reference) (NormalImpulse :type Vector :default "0, 0, 0") (Hit :type Hit%20Result%20Structure%20%28by%20ref%29))
  (Variables|Default|SetIsBeingMined true))

(event Custom|Mine
  (Utilities|FlowControl|Delay 0.2)
  (Variables|Default|SetHealth (- (Variables|Default|GetHealth) 1)))

(event EventBeginPlay
  (Variables|Default|SetHealth 10))

(event Collision|EventActorBeginOverlap
  (params (OtherActor :type Actor%20Object%20Reference)))

(event EventTick
  (params (DeltaSeconds :type Float%20%28single-precision%29))
  (if (Variables|Default|GetIsBeingMined)
    (CallFunction|Mine)
    (if (== (Variables|Default|GetHealth) 0)
      (Development|PrintText "Drop Items")
      (Actor|DestroyActor))))

(fn ConstructionScript)
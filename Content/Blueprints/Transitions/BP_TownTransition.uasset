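; BP_TownTransition is a trigger box that moves the player from the camp to town by opening the Map_test level, gated on tutorial progress.
; On overlap it reads TutorialJoeEventNumber from GI_PlayerData; once high enough, it advances that counter within a narrow range and records the transition location before loading.
; Otherwise it shows a UI_Warning widget, which is removed when the overlap ends.
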(event OnComponentBeginOverlap(Box)
  (params (OverlappedComponent :type Primitive%20Component%20Object%20Reference) (OtherActor :type Actor%20Object%20Reference) (OtherComp :type Primitive%20Component%20Object%20Reference) (OtherBodyIndex :type Integer) (bFromSweep :type Boolean) (SweepResult :type Hit%20Result%20Structure%20%28by%20ref%29))
  (bind _asgi_player_data (Utilities|Casting|CastToGI_PlayerData (Game|GetGameInstance)))
  (if (>= (Variables|/Game/Blueprints/GI_PlayerData.GI_PlayerData_C|GetTutorialJoeEventNumber _asgi_player_data) 14)
    (if (<= (Variables|/Game/Blueprints/GI_PlayerData.GI_PlayerData_C|GetTutorialJoeEventNumber _asgi_player_data) 16)
      (Variables|/Game/Blueprints/GI_PlayerData.GI_PlayerData_C|SetTutorialJoeEventNumber _asgi_player_data (+ (Variables|/Game/Blueprints/GI_PlayerData.GI_PlayerData_C|GetTutorialJoeEventNumber _asgi_player_data) 1)))
    (Variables|/Game/Blueprints/GI_PlayerData.GI_PlayerData_C|SetLastTransitionLocation _asgi_player_data "CampsTownTransition")
    (Game|OpenLevel(byName) "Map_test")
    (else
      (bind _returnvalue (UserInterface|CreateWidget "/Game/UI/UI_Warning.UI_Warning_C"))
      (UserInterface|Viewport|AddtoViewport _returnvalue 0))))

(event OnComponentEndOverlap(Box)
  (params (OverlappedComponent :type Primitive%20Component%20Object%20Reference) (OtherActor :type Actor%20Object%20Reference) (OtherComp :type Primitive%20Component%20Object%20Reference) (OtherBodyIndex :type Integer))
  (Utilities|IsValid (stale OnComponentBeginOverlap(Box) _returnvalue)
    (:Is%20Valid
      (Widget|RemovefromParent (stale OnComponentBeginOverlap(Box) _returnvalue)))))

(event EventBeginPlay)

(event Collision|EventActorBeginOverlap
  (params (OtherActor :type Actor%20Object%20Reference)))

(event EventTick
  (params (DeltaSeconds :type Float%20%28single-precision%29)))

(fn ConstructionScript)
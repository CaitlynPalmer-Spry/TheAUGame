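; BP_Item is a world item actor that displays a 2D item material from its Item data on the AnItem component.
; The construction script applies that material and enables physics simulation.
; On BeginPlay it shrinks the component for Pickaxe, Pistol and Newspaper items, leaving Gold unscaled.
; It then teleports the component by a local offset derived from the GameState actor's location, lowered along Z.
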(event EventBeginPlay
  (bind _anitem (Variables|Default|GetAnItem))
  (switch string (Utilities|String|ToString(Text) (.Name (Utilities|Struct|BreakS_ItemStructure (Variables|Default|GetItem))))
    (:Default
      _)
    (:Pickaxe
      (Transformation|SetRelativeScale3D _anitem "0.330000,0.330000,0.330000" :!label _label))
    (:Gold
      _)
    (:Pistol
      (goto _label))
    (:Newspaper
      (goto _label)))
  (Transformation|AddLocalOffset _anitem (- (Transformation|GetActorLocation (Game|GetGameState)) "0.000000,0.000000,25.000000") false true))

(event Collision|EventActorBeginOverlap
  (params (OtherActor :type Actor%20Object%20Reference)))

(event EventTick
  (params (DeltaSeconds :type Float%20%28single-precision%29)))

(fn ConstructionScript
  (bind _anitem (Variables|Default|GetAnItem))
  (Rendering|Material|SetMaterial _anitem 0 (.2d_Item (Utilities|Struct|BreakS_ItemStructure (Variables|Default|GetItem))))
  (Physics|SetSimulatePhysics _anitem true))